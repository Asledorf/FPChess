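; ChessPlayer is a player controller that lets the player click on a chess board with the mouse.
; On begin play it shows the cursor and caches the first Chess actor in the level as the board.
; On left mouse release it traces under the cursor on the Visibility channel, and if the hit component belongs to that board, passes the component's relative location to the board's OnClick.
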(event EventBeginPlay
  (Variables|Default|SetbShowMouseCursor true)
  (bind _outactors (Actor|GetAllActorsOfClass "/Game/Blueprints/Chess/Chess.Chess_C"))
  (Variables|Default|SetChessBoard (Utilities|Array|Get(acopy) _outactors)))

(event Input|MouseEvents|LeftMouseButton
  (params (Key :type Key%20Structure :default "None"))
  (bind _hitresult (Game|Player|GetHitResultUnderCursorbyChannel "TraceTypeQuery1" true))
  (bind _chessboard (Variables|Default|GetChessBoard))
  (bind _hitcomponent (Collision|BreakHitResult _hitresult))
  (:Released
    (if (== _chessboard (Components|GetOwner _hitcomponent))
      (Default|OnClick _chessboard (Variables|/Script/Engine.SceneComponent|GetRelativeLocation _hitcomponent)))))

(fn ConstructionScript)