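; Chess board Blueprint that builds squares and pieces in the construction script and handles click-to-move play.
; A 64-index loop adds checkered square meshes and pieces typed by BordInit, stored in parallel Board and Pieces arrays.
; OnClick converts positions to indices: the first click selects and highlights a piece, the next moves it, destroying any occupant.
; Move legality and turn order are not enforced; ValidMove is an uncalled stub.
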(fn ConstructionScript
  (CallFunction|GenerateBoard))

(fn GenerateBoard
  (for _index (range 0 63)
    (Utilities|FlowControl|Sequence
      (:then_0
        (|SetupBoard (Math|Conversions|ToTransform(Vector) (Utilities|IndextoPosition _index)) _index))
      (:then_1
        (|SetupPieces (Math|Conversions|ToTransform(Vector) (Utilities|IndextoPosition _index)) _index)))))

(fn OnClick
  (params (Position :type Vector))
  (bind _returnvalue (Utilities|PositiontoIndex Position))
  (bind _current_piece (Variables|Default|GetCurrent%20Piece))
  (bind _pieces (Variables|Default|Getpieces))
  (bind _output (Utilities|Array|Get(acopy) _pieces _returnvalue))
  (if (== (Variables|Default|Getlast_clicked) -1) ; IS this the piece selection click?
    (|SelectPiece _returnvalue)
    (else
      (Utilities|IsValid _output
        (:Is%20Valid
          (Components|DestroyComponent _output))
        (:Is%20Not%20Valid
          _))
      (Transformation|SetRelativeLocation _current_piece Position false false)
      (Utilities|Array|SetArrayElem (Variables|Default|Getpieces) _returnvalue _current_piece)
      (Utilities|Array|SetArrayElem (Variables|Default|Getpieces) (Variables|Default|Getlast_clicked) 0)
      ;[0 0.8828 1] reset board material
      (Rendering|Material|SetMaterial (Utilities|Array|Get(acopy) (Variables|Default|Getboard) (Variables|Default|Getlast_clicked)) 0 (Utilities|IndextoSquareMaterial (Variables|Default|Getlast_clicked)))
      (Variables|Default|Setlast_clicked -1))))

(fn ValidMove
  (if true ; If move is not valid, do nothing
    (return)))