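; Chess board anchor Blueprint that keeps the player's DefaultPawn within a spherical boundary around the world origin.
; BeginPlay caches the first DefaultPawn found as Player, and Tick repeats that lookup whenever the reference is invalid.
; Each Tick, a pawn farther than MaxDistance is moved back onto the sphere along its direction from the origin, without sweeping.
; The anchor's own location plays no part in the clamp.
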(event EventBeginPlay
  (bind _outactors (Actor|GetAllActorsOfClass "/Script/Engine.DefaultPawn"))
  (Variables|Default|SetPlayer (Utilities|Array|Get(acopy) _outactors)))

(event EventTick
  (params (DeltaSeconds :type Float%20%28single-precision%29))
  (bind _max_distance (Variables|Default|GetMax%20Distance))
  (if (Utilities|IsValid (Variables|Default|GetPlayer))
    (if (< _max_distance (Math|Vector|VectorLength (Transformation|GetActorLocation (Variables|Default|GetPlayer))))
      (Transformation|SetActorLocation (Variables|Default|GetPlayer) (* (Math|Vector|Normalize (Transformation|GetActorLocation (Variables|Default|GetPlayer)) 0.0) _max_distance) false false))
    (else
      (bind _outactors (Actor|GetAllActorsOfClass "/Script/Engine.DefaultPawn"))
      (Variables|Default|SetPlayer (Utilities|Array|Get(acopy) _outactors)))))

(fn ConstructionScript)