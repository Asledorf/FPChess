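; Gun Blueprint that fires projectile actors from its barrel tip, with a configurable shot count, spread angle and speed.
; Shoot repeatedly calls SpawnBullet, which spawns the Ammo class at BarrelTip in a random direction within the spread cone.
; Each bullet's Projectile velocity is set along its forward vector, scaled by ShotSpeed.
; Reload is an empty stub.
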(fn ConstructionScript)

(fn Shoot
  (for _index (range 0 (Variables|Default|GetShotAmount))
    (Utilities|SpawnBullet (Variables|Default|GetShotSpreadAngle))))

(fn Reload)