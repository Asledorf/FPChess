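; Map generator Blueprint that builds an 8x8 board of static mesh pieces in its Construction Script.
; GenerateBoard loops over 64 indices, converts each to a grid position and passes it to SetupPieces.
; SetupPieces adds a mesh component there, choosing plane, sphere, cube or cylinder from the BordInit entry.
; Helper graphs define index-position conversion on a 100-unit grid and checkerboard material selection, though SetupPieces applies no material.
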(fn ConstructionScript
  (CallFunction|GenerateBoard))

(fn GenerateBoard
  (for _index (range 0 63)
    (|SetupPieces (Math|Conversions|ToTransform(Vector) (Utilities|IndextoPosition _index)) _index)))